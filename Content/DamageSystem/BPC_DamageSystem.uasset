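; BPC_DamageSystem is an actor component that tracks health, invincibility and death for its owner.
; TakeDamage runs CanBeDamaged, which blocks hits on dead or invincible owners unless the damage info pierces invincibility.
; An accepted hit subtracts health, sends a knockback message to the owner, and at zero health sets IsDead and calls the OnDeath dispatcher.
; TakeDamage returns whether damage was applied.
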(event EventBeginPlay)

(event EventTick
  (params (DeltaSeconds :type Float%20%28single-precision%29)))

(fn TakeDamage
  (params (DamageInfo :type S%20Damage%20Info%20Structure))
  (bind (_amount _damagetype _damageresponse _pierceinvincible _knockbackdirection _knockbackamount) (Utilities|Struct|BreakS_DamageInfo DamageInfo))
  (Utilities|CanbeDamaged _pierceinvincible
    (:ApplyDamage
      (if (not (Variables|Default|GetIsDead))
        (bind _output_get (Variables|Default|SetCurrentHealth (- (Variables|Default|GetCurrentHealth) _amount)))
        (Class|BPIDamageable|GetKnockedBack(Message) (Components|GetOwner) (* _knockbackdirection _knockbackamount))
        (if (<= _output_get 0.0)
          (Variables|Default|SetIsDead true)
          (Default|CallOnDeath))
        (return true)))
    (:NoDamage
      (return false))))